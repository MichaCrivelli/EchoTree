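; BP_EndItem is an overlap-triggered end item that either switches the game to the echo world or ends play, depending on the current world state.
; On overlap it caches the player controller and character, then checks IsEchoVisible on GM_Main.
; If the echo world is hidden, it plays a screen fade and calls ShowEchoWorld after a short delay.
; If already visible, it disables character movement and shows the WBPGwunne widget.
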(event EventBeginPlay)

(event EventTick
  (params (DeltaSeconds :type Float%20%28single-precision%29)))

(event Collision|EventActorBeginOverlap
  (params (OtherActor :type Actor%20Object%20Reference))
  (bind _asbp_third_person_player_controller (Utilities|Casting|CastToBP_ThirdPersonPlayerController (Game|GetPlayerController 0))
    (:then
      (Variables|Default|SetPC _asbp_third_person_player_controller))
    (:CastFailed
      _))
  (bind _asbp_third_person_character (Utilities|Casting|CastToBP_ThirdPersonCharacter OtherActor)
    (:then
      (Variables|Default|SetAs%20BP%20Third%20Person%20Character _asbp_third_person_character))
    (:CastFailed
      _))
  (bind _asgm_main (Utilities|Casting|CastToGM_Main (Game|GetGameMode)))
  (Variables|Default|SetAs%20GM%20Main _asgm_main)
  (if (Variables|/Game/GameCore/GM_Main.GM_Main_C|GetIsEchoVisible (Variables|Default|GetAs%20GM%20Main))
    (Pawn|Components|CharacterMovement|DisableMovement (Variables|/Script/Engine.Character|GetCharacterMovement _asbp_third_person_character))
    (Widget|SetVisibility (Variables|/Game/UI/WBP_Ingame.WBP_Ingame_C|GetWBP_Gwunne (Variables|/Game/ThirdPerson/Blueprints/BP_ThirdPersonPlayerController.BP_ThirdPersonPlayerController_C|GetWidget _asbp_third_person_player_controller)) "Visible")
    (else
      (UserInterface|Animation|PlayAnimation (Variables|/Game/UI/WBP_Ingame.WBP_Ingame_C|GetWBP_FadeScreen (Variables|/Game/ThirdPerson/Blueprints/BP_ThirdPersonPlayerController.BP_ThirdPersonPlayerController_C|GetWidget (Variables|Default|GetPC))) (Variables|/Game/UI/WBP_FadeScreen.WBP_FadeScreen_C|GetFade (Variables|/Game/UI/WBP_Ingame.WBP_Ingame_C|GetWBP_FadeScreen (Variables|/Game/ThirdPerson/Blueprints/BP_ThirdPersonPlayerController.BP_ThirdPersonPlayerController_C|GetWidget (Variables|Default|GetPC)))) 0.0 1 "Forward" 1.0 false)
      (Utilities|FlowControl|Delay 0.4)
      (Default|ShowEchoWorld (Variables|Default|GetAs%20GM%20Main) true))))

(fn ConstructionScript)