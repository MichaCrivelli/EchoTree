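; BP_SchwingendiAxt is a swinging axe object that rocks back and forth continuously like a pendulum.
; Each tick it sets the mesh's world pitch to a sine of game time, with Schwinggschwindigkeit as the speed and Schwingwinkel as the angle amplitude.
; Roll and yaw are forced to zero, so placed rotation of the mesh is overridden.
; The Blueprint has no overlap or damage logic.
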(event EventBeginPlay
  (|CallParentFunction) ; This node is disabled and will not be called.\nDrag off pins to build functionality.
)

(event Collision|EventActorBeginOverlap
  (params (OtherActor :type Actor%20Object%20Reference))
  (|CallParentFunction OtherActor) ; This node is disabled and will not be called.\nDrag off pins to build functionality.
)

(event EventTick
  (params (DeltaSeconds :type Float%20%28single-precision%29))
  (|CallParentFunction DeltaSeconds)
  (Transformation|SetWorldRotation (Variables|Character|GetMesh) (Math|Rotator|MakeRotator 0.0 (* (Math|Trig|Sin(Radians) (* (Variables|Default|GetSchwinggschwindigkeit) (Utilities|Time|GetGameTimeinSeconds))) (Variables|Default|GetSchwingwinkel)) 0.0) false false))

(fn ConstructionScript
  (|CallParentFunction))