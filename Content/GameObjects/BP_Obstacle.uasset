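; Obstacle actor that reacts when the third-person character overlaps its mesh, either revealing the echo world or restarting the character.
; After a short delay it increments the character's hit count, then checks echo visibility on GM_Main.
; A visible echo triggers a restart that ends replay and restores Blueprint animation; otherwise the screen fade plays before the echo world appears.
; Separate events re-enable mesh collision and swap between default and ability materials.
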(event OnComponentBeginOverlap(Mesh)
  (params (OverlappedComponent :type Primitive%20Component%20Object%20Reference) (OtherActor :type Actor%20Object%20Reference) (OtherComp :type Primitive%20Component%20Object%20Reference) (OtherBodyIndex :type Integer) (bFromSweep :type Boolean) (SweepResult :type Hit%20Result%20Structure%20%28by%20ref%29))
  (bind _gm_main (Variables|Default|GetGM_Main))
  (bind _asbp_third_person_character (Utilities|Casting|CastToBP_ThirdPersonCharacter OtherActor))
  (Utilities|FlowControl|Delay 0.2)
  (Math|Integer|IncrementInt (Variables|/Game/ThirdPerson/Blueprints/BP_ThirdPersonCharacter.BP_ThirdPersonCharacter_C|GetObstaclesHit _asbp_third_person_character)
    (:%20%20
      (if (Variables|/Game/GameCore/GM_Main.GM_Main_C|GetIsEchoVisible _gm_main)
        (Default|Restart _asbp_third_person_character)
        (Variables|/Game/ThirdPerson/Blueprints/BP_ThirdPersonCharacter.BP_ThirdPersonCharacter_C|SetIsReplaying _asbp_third_person_character false)
        (Components|Animation|SetAnimationMode (Variables|/Script/Engine.Character|GetMesh _asbp_third_person_character) "AnimationBlueprint" true)
        (else
          (bind _asbp_third_person_player_controller (Utilities|Casting|CastToBP_ThirdPersonPlayerController (Game|GetPlayerController 0)))
          (UserInterface|Animation|PlayAnimation (Variables|/Game/UI/WBP_Ingame.WBP_Ingame_C|GetWBP_FadeScreen (Variables|/Game/ThirdPerson/Blueprints/BP_ThirdPersonPlayerController.BP_ThirdPersonPlayerController_C|GetWidget _asbp_third_person_player_controller)) (Variables|/Game/UI/WBP_FadeScreen.WBP_FadeScreen_C|GetFade (Variables|/Game/UI/WBP_Ingame.WBP_Ingame_C|GetWBP_FadeScreen (Variables|/Game/ThirdPerson/Blueprints/BP_ThirdPersonPlayerController.BP_ThirdPersonPlayerController_C|GetWidget _asbp_third_person_player_controller))) 0.0 1 "Forward" 1.0 false)
          (Utilities|FlowControl|Delay 0.4)
          (Default|ShowEchoWorld _gm_main true))))))

(event Custom|ResetCollision
  (Collision|SetCollisionEnabled (Variables|Default|GetMesh) "QueryAndPhysics"))

(event Custom|ChangeMaterial
  (params (IsAbilityMat :type Boolean))
  (bind _mesh (Variables|Default|GetMesh))
  (if IsAbilityMat
    (Rendering|Material|SetMaterial _mesh 0 (Variables|Default|GetAbility%20Material))
    (else
      (Rendering|Material|SetMaterial _mesh 0 (Variables|Default|GetDefault%20Material)))))

(event Collision|EventActorBeginOverlap
  (params (OtherActor :type Actor%20Object%20Reference)))

(event EventTick
  (params (DeltaSeconds :type Float%20%28single-precision%29)))

(event EventBeginPlay
  (bind _asgm_main (Utilities|Casting|CastToGM_Main (Game|GetGameMode)))
  (Variables|Default|SetGM_Main _asgm_main))

(fn ConstructionScript)