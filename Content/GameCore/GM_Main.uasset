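; GM_Main is the game mode that manages switching between the Happy and Echo worlds and tracks remaining tries.
; On BeginPlay it streams in both worlds and their separate obstacle levels, showing only Happy.
; ShowEchoWorld flips level visibility, resets transition and obstacle collision, and broadcasts real switches.
; The See Echo ability toggles Echo obstacle visibility, then after a brief delay swaps tagged obstacles' materials.
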(event Custom|TriggerAbilitySeeEcho
  (params (IsActive :type Boolean))
  (Variables|/Script/Engine.LevelStreaming|SetbShouldBeVisible (Variables|Default|GetEchoObstacles) IsActive)
  (Utilities|FlowControl|Delay 0.05)
  (CallFunction|AbilitySeeEchoObstacles IsActive))

(event EventBeginPlay
  (Class|GameplayStatics|LoadStreamLevelbySoftObjectPtr "/Game/Levels/HappyWorld.HappyWorld" true false)
  (Class|GameplayStatics|LoadStreamLevelbySoftObjectPtr "/Game/Levels/HappyObstacles.HappyObstacles" true false)
  (Class|GameplayStatics|LoadStreamLevelbySoftObjectPtr "/Game/Levels/EchoObstacles.EchoObstacles" false false)
  (Class|GameplayStatics|LoadStreamLevelbySoftObjectPtr "/Game/Levels/EchoWorld.EchoWorld" false false)
  (Variables|Default|SetHappyWorld (Class|GameplayStatics|GetStreamingLevel "HappyWorld"))
  (Variables|Default|SetEchoWorld (Class|GameplayStatics|GetStreamingLevel "EchoWorld"))
  (Variables|Default|SetHappyObstacles (Class|GameplayStatics|GetStreamingLevel "HappyObstacles"))
  (Variables|Default|SetEchoObstacles (Class|GameplayStatics|GetStreamingLevel "EchoObstacles")))

(fn ConstructionScript)

(fn ShowEchoWorld
  (params (Show :type Boolean))
  (bind _returnvalue (not Show))
  (if (!= Show (Variables|Default|GetIsEchoVisible))
    (Variables|Default|SetIsEchoVisible Show)
    (Variables|/Script/Engine.LevelStreaming|SetbShouldBeVisible (Variables|Default|GetEchoWorld) Show)
    (Variables|/Script/Engine.LevelStreaming|SetbShouldBeVisible (Variables|Default|GetEchoObstacles) Show)
    (Variables|/Script/Engine.LevelStreaming|SetbShouldBeVisible (Variables|Default|GetHappyWorld) _returnvalue)
    (Variables|/Script/Engine.LevelStreaming|SetbShouldBeVisible (Variables|Default|GetHappyObstacles) _returnvalue)
    (bind _outactors (Actor|GetAllActorsOfClass "/Game/GameObjects/BP_TransitionToEcho.BP_TransitionToEcho_C"))
    (for _array_element _outactors
      (Default|ResetCollision _array_element))
    (bind _outactors_2 (Actor|GetAllActorsOfClass "/Game/GameObjects/BP_Obstacle.BP_Obstacle_C"))
    (for _array_element_2 _outactors_2
      (Default|ResetCollision _array_element_2))
    (Default|CallWorldSwitch Show)
    (else
      (bind _outactors_3 (Actor|GetAllActorsOfClass "/Game/GameObjects/BP_TransitionToEcho.BP_TransitionToEcho_C"))
      (for _array_element_3 _outactors_3
        (Default|ResetCollision _array_element_3))
      (bind _outactors_4 (Actor|GetAllActorsOfClass "/Game/GameObjects/BP_Obstacle.BP_Obstacle_C"))
      (for _array_element_4 _outactors_4
        (Default|ResetCollision _array_element_4)))))

(fn RemoveTry
  (bind _result (Math|Integer|DecrementInt (Variables|Default|GetTriesLeft))
    (:%20%20
      (if (<= _result 0)
        (Default|CallOnAllTriesUsed)))))

(fn AbilitySeeEchoObstacles
  (params (IsActive :type Boolean))
  (bind _outactors (Actor|GetAllActorsOfClasswithTag "/Game/GameObjects/BP_Obstacle.BP_Obstacle_C" "echo"))
  (Variables|Default|SetAllEchoObstacles _outactors)
  (if IsActive
    (for _array_element (Variables|Default|GetAllEchoObstacles)
      (Default|ChangeMaterial _array_element true)
      (Development|PrintString "abi mat"))
    (else
      (for _array_element_2 (Variables|Default|GetAllEchoObstacles)
        (Default|ChangeMaterial _array_element_2 false)))))